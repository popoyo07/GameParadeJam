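; BP_Target is a shootable target actor that scores a hit when a bullet overlaps it.
; Its Collider overlap event prints a debug string, then checks whether the other actor is a BP_Bullet.
; A match increments the HitTarget counter on the ShootingLevel reference and destroys the target.
; The Destroyed event plays the TargetDestroy sound at the actor's location.
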(event OnComponentBeginOverlap(Collider)
  (params (OverlappedComponent :type Primitive%20Component%20Object%20Reference) (OtherActor :type Actor%20Object%20Reference) (OtherComp :type Primitive%20Component%20Object%20Reference) (OtherBodyIndex :type Integer) (bFromSweep :type Boolean) (SweepResult :type Hit%20Result%20Structure%20%28by%20ref%29))
  (Development|PrintString "Hello")
  (if (Class|GameplayStatics|ObjectIsA OtherActor "/Game/ActualGame/BluePrints/BP_Bullet.BP_Bullet_C")
    (Variables|/Game/ActualGame/BluePrints/LevelLogic/BP_ShootingLevel.BP_ShootingLevel_C|SetHitTarget (Variables|Default|GetShootingLevel) (+ (Variables|/Game/ActualGame/BluePrints/LevelLogic/BP_ShootingLevel.BP_ShootingLevel_C|GetHitTarget (Variables|Default|GetShootingLevel)) 1))
    (Actor|DestroyActor)))

(event EventDestroyed
  (Audio|PlaySoundatLocation "/Game/ActualGame/Sound/TargetDestroy.TargetDestroy" (Transformation|GetActorLocation) "0, 0, 0" 1.0 1.0 0.0 0 0 0 0))

(fn ConstructionScript)