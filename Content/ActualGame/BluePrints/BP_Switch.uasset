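; BP_Switch is an interactable switch that either destroys security cameras or disables a laser in the level.
; Its collision overlap events track whether BP_ThirdPersonCharacter is touching it and hand that character a reference to the switch.
; LevelInteraction destroys every valid actor in Cameras when ZachManager is valid, otherwise asks LevelManager to disable the laser.
; Both actions require the touching flag, and the character's switch reference stays set after overlap ends.
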(event OnComponentBeginOverlap(Collisio)
  (params (OverlappedComponent :type Primitive%20Component%20Object%20Reference) (OtherActor :type Actor%20Object%20Reference) (OtherComp :type Primitive%20Component%20Object%20Reference) (OtherBodyIndex :type Integer) (bFromSweep :type Boolean) (SweepResult :type Hit%20Result%20Structure%20%28by%20ref%29))
  (bind _asbp_third_person_character (Utilities|Casting|CastToBP_ThirdPersonCharacter OtherActor))
  (Variables|Default|SetTouching%20Switch true)
  (Development|PrintString "Touching")
  (Variables|/Game/ThirdPerson/Blueprints/BP_ThirdPersonCharacter.BP_ThirdPersonCharacter_C|SetSwitch%20 _asbp_third_person_character self))

(event OnComponentEndOverlap(Collisio)
  (params (OverlappedComponent :type Primitive%20Component%20Object%20Reference) (OtherActor :type Actor%20Object%20Reference) (OtherComp :type Primitive%20Component%20Object%20Reference) (OtherBodyIndex :type Integer))
  (Utilities|Casting|CastToBP_ThirdPersonCharacter OtherActor)
  (Variables|Default|SetTouching%20Switch false)
  (Development|PrintString "Not touching"))

(event Custom|Level%20Interaction
  (Utilities|IsValid (Variables|Default|GetZach%20Manager)
    (:Is%20Valid
      (CallFunction|DestroyCameras))
    (:Is%20Not%20Valid
      (if (Variables|Default|GetTouching%20Switch)
        (Default|DsableLaser (Variables|Default|GetLevel%20Manager))))))

(event Custom|Destroy%20Cameras
  (bind _cameras (Variables|Default|GetCameras))
  (if (Variables|Default|GetTouching%20Switch)
    (for (_ _array_index) _cameras
      (Utilities|IsValid (Utilities|Array|Get(acopy) _cameras _array_index)
        (:Is%20Valid
          _)
        (:Is%20Not%20Valid
          (Utilities|IsValid (Utilities|Array|Get(acopy) _cameras _array_index)
            (:Is%20Valid
              _))))
      (Actor|DestroyActor (Utilities|Array|Get(acopy) _cameras _array_index)))))

(event EventBeginPlay)

(event Collision|EventActorBeginOverlap
  (params (OtherActor :type Actor%20Object%20Reference)))

(fn ConstructionScript)