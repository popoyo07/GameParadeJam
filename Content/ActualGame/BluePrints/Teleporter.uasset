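; Teleporter actor that moves the player to a target actor's location in exchange for a card.
; Overlapping its Box stores the BP_ThirdPersonCharacter as Player, a reference that is never cleared on leaving.
; Tick polls that player's PressedE and HasCard flags, then calls RemoveItem and teleports them to TpPos with zero rotation.
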(event OnComponentBeginOverlap(Box)
  (params (OverlappedComponent :type Primitive%20Component%20Object%20Reference) (OtherActor :type Actor%20Object%20Reference) (OtherComp :type Primitive%20Component%20Object%20Reference) (OtherBodyIndex :type Integer) (bFromSweep :type Boolean) (SweepResult :type Hit%20Result%20Structure%20%28by%20ref%29))
  (bind _asbp_third_person_character (Utilities|Casting|CastToBP_ThirdPersonCharacter OtherActor))
  (Variables|Default|SetPlayer _asbp_third_person_character))

(event EventBeginPlay)

(event Collision|EventActorBeginOverlap
  (params (OtherActor :type Actor%20Object%20Reference)))

(event EventTick
  (params (DeltaSeconds :type Float%20%28single-precision%29))
  (bind _player (Variables|Default|GetPlayer))
  (Utilities|IsValid _player
    (:Is%20Valid
      (if (Variables|/Game/ThirdPerson/Blueprints/BP_ThirdPersonCharacter.BP_ThirdPersonCharacter_C|GetPressed%20E _player)
        (if (Variables|/Game/ThirdPerson/Blueprints/BP_ThirdPersonCharacter.BP_ThirdPersonCharacter_C|GetHasCard _player)
          (Default|RemoveItem _player)
          (Transformation|Teleport _player (Transformation|GetActorLocation (Variables|Default|Gettp%20Pos)) "0, 0, 0"))))))

(fn ConstructionScript)