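; BP_KillerLaser is a hazard actor that triggers the lose screen when the player touches it.
; Overlap on its collision component with BP_ThirdPersonCharacter opens LoseMenu, shows the mouse cursor and switches player input to UI only.
; When the laser is destroyed, it plays a disable sound at its location and also destroys its separate VFX actor.
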(event OnComponentBeginOverlap(Collidsion)
  (params (OverlappedComponent :type Primitive%20Component%20Object%20Reference) (OtherActor :type Actor%20Object%20Reference) (OtherComp :type Primitive%20Component%20Object%20Reference) (OtherBodyIndex :type Integer) (bFromSweep :type Boolean) (SweepResult :type Hit%20Result%20Structure%20%28by%20ref%29))
  (bind _returnvalue (Game|GetPlayerController 0))
  (Utilities|Casting|CastToBP_ThirdPersonCharacter OtherActor
    (:then
      (Development|PrintString "collision ")
      (bind _returnvalue_2 (Game|ConstructObjectfromClass "/Game/ActualGame/UI/LoseMenu.LoseMenu_C"))
      (UserInterface|Viewport|AddtoViewport _returnvalue_2 0)
      (Variables|/Script/Engine.PlayerController|SetbShowMouseCursor _returnvalue true)
      (Input|SetInputModeUIOnly _returnvalue 0 "DoNotLock" false))
    (:CastFailed
      (Development|PrintString "falied"))))

(event EventBeginPlay)

(event EventDestroyed
  (Audio|PlaySoundatLocation "/Game/ActualGame/Sound/Laser_Disable.Laser_Disable" (Transformation|GetActorLocation) "0, 0, 0" 1.0 1.0 0.0 0 0 0 0)
  (Actor|DestroyActor (Variables|Default|GetVFX)))

(event EventTick
  (params (DeltaSeconds :type Float%20%28single-precision%29)))

(fn ConstructionScript)