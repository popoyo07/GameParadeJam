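; BP_ShootingLevel is the shooting challenge logic actor, with a win and a lose outcome.
; Its Detect volume flags the player's presence and counts overlapping bullets, while HitTarget is only read here.
; Once the player has entered, Tick triggers CardSpawner at the target goal or the lose menu at the bullet limit.
; Entering PlayerNotAllowed also loses; either outcome destroys the actor, playing a bubble sound.
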(event OnComponentBeginOverlap(PlayerNotAllowed)
  (params (OverlappedComponent :type Primitive%20Component%20Object%20Reference) (OtherActor :type Actor%20Object%20Reference) (OtherComp :type Primitive%20Component%20Object%20Reference) (OtherBodyIndex :type Integer) (bFromSweep :type Boolean) (SweepResult :type Hit%20Result%20Structure%20%28by%20ref%29))
  (bind _returnvalue (Game|GetPlayerController 0))
  (Utilities|Casting|CastToBP_ThirdPersonCharacter OtherActor)
  ;[0.15 0.15 0.15 0.5] Enable lose screen
  (bind _returnvalue_2 (Game|ConstructObjectfromClass "/Game/ActualGame/UI/LoseMenu.LoseMenu_C"))
  (UserInterface|Viewport|AddtoViewport _returnvalue_2 0)
  (Variables|/Script/Engine.PlayerController|SetbShowMouseCursor _returnvalue true)
  (Input|SetInputModeUIOnly _returnvalue 0 "DoNotLock" false)
  (Actor|DestroyActor))

(event OnComponentBeginOverlap(Detect)
  (params (OverlappedComponent :type Primitive%20Component%20Object%20Reference) (OtherActor :type Actor%20Object%20Reference) (OtherComp :type Primitive%20Component%20Object%20Reference) (OtherBodyIndex :type Integer) (bFromSweep :type Boolean) (SweepResult :type Hit%20Result%20Structure%20%28by%20ref%29))
  (Development|PrintString "overlap")
  (Utilities|Casting|CastToBP_ThirdPersonCharacter OtherActor
    (:then
      (bind _output_get (Variables|Default|Setoverlap%20Player true)))
    (:CastFailed
      ;[0.15 0.15 0.15 0.5] Bullet counter
      (Utilities|Casting|CastToBP_Bullet OtherActor)
      (bind _output_get_2 (Variables|Default|SetBulletsShot (+ (Variables|Default|GetBulletsShot) 1)))
      (Development|PrintString (Utilities|String|ToString(Integer) _output_get_2)))))

(event EventBeginPlay)

(event Collision|EventActorBeginOverlap
  (params (OtherActor :type Actor%20Object%20Reference)))

(event EventTick
  (params (DeltaSeconds :type Float%20%28single-precision%29))
  (bind _returnvalue (Game|GetPlayerController 0))
  (if (stale OnComponentBeginOverlap(Detect) _output_get)
    (if (== (Variables|Default|GetBulletsShot) 25)
      ;[0.15 0.15 0.15 0.5] Enable lose screen
      (bind _returnvalue_2 (Game|ConstructObjectfromClass "/Game/ActualGame/UI/LoseMenu.LoseMenu_C"))
      (UserInterface|Viewport|AddtoViewport _returnvalue_2 0)
      (Variables|/Script/Engine.PlayerController|SetbShowMouseCursor _returnvalue true)
      (Input|SetInputModeUIOnly _returnvalue 0 "DoNotLock" false)
      (Actor|DestroyActor)
      (else
        (Development|PrintString (Utilities|String|ToString(Integer) (Variables|Default|GetHitTarget)))
        ;[0.15 0.15 0.15 0.5] Place door bp reference after this
        (if (== (Variables|Default|GetHitTarget) 6)
          (Default|CardSpawner (Variables|Default|GetCardSpawner))
          (Actor|DestroyActor))))))

(event EventDestroyed
  (Audio|PlaySound2D "/Game/ActualGame/Sound/bubble-sound-43207.bubble-sound-43207" 1.0 1.0 0.0 0 0))

(fn ConstructionScript)