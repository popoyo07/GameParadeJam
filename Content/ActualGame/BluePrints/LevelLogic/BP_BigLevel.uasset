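; BP_BigLevel is a level-logic actor that tracks puzzle locks for a gate and can disable a laser.
; Tick waits for ShootingLocks and OrbLocks to both equal two, then calls the empty UnlockGate event and destroys the actor.
; Both 2orbsthingy and ShootingDefuse increment OrbLocks; nothing here changes ShootingLocks.
; Its box overlap passes TheSwitch to the player character, and Dsablelaser destroys the Laser.
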(event OnComponentBeginOverlap(Box)
  (params (OverlappedComponent :type Primitive%20Component%20Object%20Reference) (OtherActor :type Actor%20Object%20Reference) (OtherComp :type Primitive%20Component%20Object%20Reference) (OtherBodyIndex :type Integer) (bFromSweep :type Boolean) (SweepResult :type Hit%20Result%20Structure%20%28by%20ref%29))
  (bind _asbp_third_person_character (Utilities|Casting|CastToBP_ThirdPersonCharacter OtherActor))
  (Development|PrintString "Begiin overlap")
  (Variables|/Game/ThirdPerson/Blueprints/BP_ThirdPersonCharacter.BP_ThirdPersonCharacter_C|SetSwitch%20 _asbp_third_person_character (Variables|Default|GetTheSwitch)))

(event Custom|Dsable%20laser
  (Actor|DestroyActor (Variables|Default|GetLaser))
  (Development|PrintString "Laser Dsabled"))

(event Custom|2%20orbs%20thingy
  (Variables|Default|SetOrb%20Locks (+ (Variables|Default|GetOrb%20Locks) 1)))

(event Custom|Shooting%20Defuse
  (Variables|Default|SetOrb%20Locks (+ (Variables|Default|GetOrb%20Locks) 1)))

(event Custom|Unlock%20Gate)

(event EventBeginPlay)

(event EventTick
  (params (DeltaSeconds :type Float%20%28single-precision%29))
  (if (== (Variables|Default|GetShooting%20Locks) 2)
    (if (== (Variables|Default|GetOrb%20Locks) 2)
      (CallFunction|UnlockGate)
      (Actor|DestroyActor))))

(fn ConstructionScript)