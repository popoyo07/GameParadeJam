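; BP_Camera_Rotating is a camera actor that sweeps back and forth in yaw while CamerasOn is true.
; Tick rotates the actor by Rotation scaled by delta time and accumulates the absolute angle, reversing direction each time it reaches a fixed limit.
; When CamerasOn is false, rotation stops and Tick deactivates the CameraLight and Cone components, with no reactivation in this graph.
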(event EventTick
  (params (DeltaSeconds :type Float%20%28single-precision%29))
  ;[0.15 0.15 0.15 0.5] Camera Rotation
  (if (Variables|Default|GetCamerasOn)
    (Transformation|AddActorLocalRotation (Math|Rotator|MakeRotator 0.0 0.0 (* DeltaSeconds (Variables|Default|GetRotation))) false false)
    (bind _output_get (Variables|Default|SetRotatationProgress (+ (Math|Float|Absolute(Float) (* DeltaSeconds (Variables|Default|GetRotation))) (Variables|Default|GetRotatationProgress))))
    (if (>= _output_get 6e+01)
      (Variables|Default|SetRotatationProgress 0.0)
      (Variables|Default|SetRotation (* -1.0 (Variables|Default|GetRotation))))
    (else
      (Components|Activation|Deactivate (Variables|Default|GetCameraLight)))))

(fn ConstructionScript
  (|CallParentFunction))