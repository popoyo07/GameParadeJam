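; BP_Camera is a security camera that detects characters entering its Cone component.
; While CamerasOn is true, an overlap by any Character sets PlayerDetected and prints it, and nothing here clears the flag.
; While CamerasOn is false, Tick calls Deactivate on the CameraLight and Cone every frame, with no reactivation path in this Blueprint.
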(event OnComponentBeginOverlap(Cone)
  (params (OverlappedComponent :type Primitive%20Component%20Object%20Reference) (OtherActor :type Actor%20Object%20Reference) (OtherComp :type Primitive%20Component%20Object%20Reference) (OtherBodyIndex :type Integer) (bFromSweep :type Boolean) (SweepResult :type Hit%20Result%20Structure%20%28by%20ref%29))
  ;[0.15 0.15 0.15 0.5] Player Detection
  (if (Variables|Default|GetCamerasOn)
    (bind _output_get (Variables|Default|SetActorIsPlayer (Class|GameplayStatics|ObjectIsA OtherActor "/Script/Engine.Character")))
    (if _output_get
      (bind _output_get_2 (Variables|Default|SetPlayerDetected true))
      (Development|PrintString (Utilities|String|ToString(Boolean) _output_get_2)))))

(event EventTick
  (params (DeltaSeconds :type Float%20%28single-precision%29))
  ;[0.15 0.15 0.15 0.5] Player Detection
  (if (not (Variables|Default|GetCamerasOn))
    (Components|Activation|Deactivate (Variables|Default|GetCameraLight))))

(fn ConstructionScript)