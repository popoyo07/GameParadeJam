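; Manager Blueprint that randomizes teleporter destinations once at BeginPlay.
; RandomizeOrder shuffles the Possibility array and uses its first element to pick one of four hardcoded scenarios.
; Scenarios 2–4 each assign waypoints to the TpPos of four teleporters in a fixed permutation, while Scenario1's loop covers only index 0.
; Each scenario prints a debug string naming the chosen layout.
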(event Custom|Randomize%20Order
  (Utilities|Array|Shuffle (Variables|Default|GetPossibility))
  (switch int (Utilities|Array|Get(acopy) (Variables|Default|GetPossibility))
    (:0
      (CallFunction|Scenario1))
    (:1
      (CallFunction|Scenario2))
    (:2
      (CallFunction|Scenario3))
    (:3
      (CallFunction|Scenario4))))

(event Custom|Scenario%201
  (for _index (range 0 0)
    (bind _output_get (Variables|Default|SetTeleporter%20 (Utilities|Array|Get(acopy) (Variables|Default|GetBp_Teleporter) _index)))
    (Variables|/Game/ActualGame/BluePrints/Teleporter.Teleporter_C|Settp%20Pos _output_get (Utilities|Array|Get(acopy) (Variables|Default|GetWaypoint) _index))
    (Development|PrintString "scenraio 1" true true "(R=0.000000,G=0.660000,B=1.000000,A=1.000000)" 1e+01)))

(event Custom|Scenario%202
  (bind _output_get (Variables|Default|SetTeleporter%20 (Utilities|Array|Get(acopy) (Variables|Default|GetBp_Teleporter))))
  (Variables|/Game/ActualGame/BluePrints/Teleporter.Teleporter_C|Settp%20Pos _output_get (Utilities|Array|Get(acopy) (Variables|Default|GetWaypoint) 1))
  (bind _output_get_2 (Variables|Default|SetTeleporter%20 (Utilities|Array|Get(acopy) (Variables|Default|GetBp_Teleporter) 1)))
  (Variables|/Game/ActualGame/BluePrints/Teleporter.Teleporter_C|Settp%20Pos _output_get_2 (Utilities|Array|Get(acopy) (Variables|Default|GetWaypoint) 3))
  (bind _output_get_3 (Variables|Default|SetTeleporter%20 (Utilities|Array|Get(acopy) (Variables|Default|GetBp_Teleporter) 2)))
  (Variables|/Game/ActualGame/BluePrints/Teleporter.Teleporter_C|Settp%20Pos _output_get_3 (Utilities|Array|Get(acopy) (Variables|Default|GetWaypoint) 2))
  (bind _output_get_4 (Variables|Default|SetTeleporter%20 (Utilities|Array|Get(acopy) (Variables|Default|GetBp_Teleporter) 3)))
  (Variables|/Game/ActualGame/BluePrints/Teleporter.Teleporter_C|Settp%20Pos _output_get_4 (Utilities|Array|Get(acopy) (Variables|Default|GetWaypoint)))
  (Development|PrintString "scenraio 2" true true "(R=0.000000,G=0.660000,B=1.000000,A=1.000000)" 1e+01))

(event Custom|Scenario%203
  (bind _output_get (Variables|Default|SetTeleporter%20 (Utilities|Array|Get(acopy) (Variables|Default|GetBp_Teleporter))))
  (Variables|/Game/ActualGame/BluePrints/Teleporter.Teleporter_C|Settp%20Pos _output_get (Utilities|Array|Get(acopy) (Variables|Default|GetWaypoint) 2))
  (bind _output_get_2 (Variables|Default|SetTeleporter%20 (Utilities|Array|Get(acopy) (Variables|Default|GetBp_Teleporter) 1)))
  (Variables|/Game/ActualGame/BluePrints/Teleporter.Teleporter_C|Settp%20Pos _output_get_2 (Utilities|Array|Get(acopy) (Variables|Default|GetWaypoint) 3))
  (bind _output_get_3 (Variables|Default|SetTeleporter%20 (Utilities|Array|Get(acopy) (Variables|Default|GetBp_Teleporter) 2)))
  (Variables|/Game/ActualGame/BluePrints/Teleporter.Teleporter_C|Settp%20Pos _output_get_3 (Utilities|Array|Get(acopy) (Variables|Default|GetWaypoint)))
  (bind _output_get_4 (Variables|Default|SetTeleporter%20 (Utilities|Array|Get(acopy) (Variables|Default|GetBp_Teleporter) 3)))
  (Variables|/Game/ActualGame/BluePrints/Teleporter.Teleporter_C|Settp%20Pos _output_get_4 (Utilities|Array|Get(acopy) (Variables|Default|GetWaypoint) 1))
  (Development|PrintString "scenraio 3" true true "(R=0.000000,G=0.660000,B=1.000000,A=1.000000)" 1e+01))

(event Custom|Scenario%204
  (bind _output_get (Variables|Default|SetTeleporter%20 (Utilities|Array|Get(acopy) (Variables|Default|GetBp_Teleporter))))
  (Variables|/Game/ActualGame/BluePrints/Teleporter.Teleporter_C|Settp%20Pos _output_get (Utilities|Array|Get(acopy) (Variables|Default|GetWaypoint) 2))
  (bind _output_get_2 (Variables|Default|SetTeleporter%20 (Utilities|Array|Get(acopy) (Variables|Default|GetBp_Teleporter) 1)))
  (Variables|/Game/ActualGame/BluePrints/Teleporter.Teleporter_C|Settp%20Pos _output_get_2 (Utilities|Array|Get(acopy) (Variables|Default|GetWaypoint) 1))
  (bind _output_get_3 (Variables|Default|SetTeleporter%20 (Utilities|Array|Get(acopy) (Variables|Default|GetBp_Teleporter) 2)))
  (Variables|/Game/ActualGame/BluePrints/Teleporter.Teleporter_C|Settp%20Pos _output_get_3 (Utilities|Array|Get(acopy) (Variables|Default|GetWaypoint) 3))
  (bind _output_get_4 (Variables|Default|SetTeleporter%20 (Utilities|Array|Get(acopy) (Variables|Default|GetBp_Teleporter) 3)))
  (Variables|/Game/ActualGame/BluePrints/Teleporter.Teleporter_C|Settp%20Pos _output_get_4 (Utilities|Array|Get(acopy) (Variables|Default|GetWaypoint)))
  (Development|PrintString "scenraio 4" true true "(R=0.000000,G=0.660000,B=1.000000,A=1.000000)" 1e+01))

(event EventBeginPlay
  (CallFunction|RandomizeOrder))

(event Collision|EventActorBeginOverlap
  (params (OtherActor :type Actor%20Object%20Reference)))

(event EventTick
  (params (DeltaSeconds :type Float%20%28single-precision%29)))

(fn ConstructionScript)