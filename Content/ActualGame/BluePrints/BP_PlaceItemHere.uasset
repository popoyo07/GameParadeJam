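; Placement spot actor that accepts up to two items from the player, shown as meshes on two slots.
; Its Box overlap registers the actor as the third-person character's PlaceItem and stores that player; end overlap only clears the Touching flag.
; PlacingItem, not called here, fills the first free slot with the Cube mesh, calls RemoveItem on the player and notifies Level through 2OrbsThingy after each placement.
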(event OnComponentBeginOverlap(Box)
  (params (OverlappedComponent :type Primitive%20Component%20Object%20Reference) (OtherActor :type Actor%20Object%20Reference) (OtherComp :type Primitive%20Component%20Object%20Reference) (OtherBodyIndex :type Integer) (bFromSweep :type Boolean) (SweepResult :type Hit%20Result%20Structure%20%28by%20ref%29))
  (bind _asbp_third_person_character (Utilities|Casting|CastToBP_ThirdPersonCharacter OtherActor))
  (Variables|/Game/ThirdPerson/Blueprints/BP_ThirdPersonCharacter.BP_ThirdPersonCharacter_C|SetPlaceItem _asbp_third_person_character self)
  (Variables|Default|SetTouching true)
  (Variables|Default|SetPlayer _asbp_third_person_character))

(event OnComponentEndOverlap(Box)
  (params (OverlappedComponent :type Primitive%20Component%20Object%20Reference) (OtherActor :type Actor%20Object%20Reference) (OtherComp :type Primitive%20Component%20Object%20Reference) (OtherBodyIndex :type Integer))
  (Utilities|Casting|CastToBP_ThirdPersonCharacter OtherActor)
  (Variables|Default|SetTouching false))

(event Custom|Placing%20Item
  (if (Variables|Default|GetTheItem1)
    (if (not (Variables|Default|GetItem2))
      (bind _returnvalue (Components|StaticMesh|SetStaticMesh (Variables|Default|Getitem2_0) "/Engine/BasicShapes/Cube.Cube"))
      (Variables|Default|SetItem2 _returnvalue)
      (Default|RemoveItem (Variables|Default|GetPlayer) :!label _label)
      (Default|2OrbsThingy (Variables|Default|GetLevel)))
    (else
      (Variables|Default|SetTheItem1 true)
      (Components|StaticMesh|SetStaticMesh (Variables|Default|GetItem1) "/Engine/BasicShapes/Cube.Cube")
      (goto _label))))

(event EventBeginPlay)

(event Collision|EventActorBeginOverlap
  (params (OtherActor :type Actor%20Object%20Reference)))

(event EventTick
  (params (DeltaSeconds :type Float%20%28single-precision%29)))

(fn ConstructionScript)