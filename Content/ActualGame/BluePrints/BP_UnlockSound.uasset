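; BP_UnlockSound is an actor that removes itself from the game once the Unlock1 flag on its Level reference is true.
; It polls that flag every Tick after a validity check on Level, then calls DestroyActor.
; Despite the name, its graphs contain no sound logic, and the construction script only calls its parent.
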(event EventBeginPlay
  (|CallParentFunction) ; This node is disabled and will not be called.\nDrag off pins to build functionality.
)

(event Collision|EventActorBeginOverlap
  (params (OtherActor :type Actor%20Object%20Reference))
  (|CallParentFunction OtherActor) ; This node is disabled and will not be called.\nDrag off pins to build functionality.
)

(event EventTick
  (params (DeltaSeconds :type Float%20%28single-precision%29))
  (bind _level (Variables|Default|GetLevel))
  (Utilities|IsValid _level
    (:Is%20Valid
      (if (Variables|/Game/ActualGame/BluePrints/LevelLogic/BP_BigLevel.BP_BigLevel_C|GetUnlock1 _level)
        (Actor|DestroyActor)))))

(fn ConstructionScript
  (|CallParentFunction))