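; BP_Door is a door actor that either teleports the player onward or, if fake, ends the game.
; Its box overlap registers the door on the third-person character and tracks whether it is touching.
; OpenDoor on a fake door shows the lose menu with UI-only input; otherwise it teleports the player to a waypoint, removes their item and can spawn a card pickup.
; Either way the door then destroys itself.
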(event OnComponentBeginOverlap(Box)
  (params (OverlappedComponent :type Primitive%20Component%20Object%20Reference) (OtherActor :type Actor%20Object%20Reference) (OtherComp :type Primitive%20Component%20Object%20Reference) (OtherBodyIndex :type Integer) (bFromSweep :type Boolean) (SweepResult :type Hit%20Result%20Structure%20%28by%20ref%29))
  (bind _asbp_third_person_character (Utilities|Casting|CastToBP_ThirdPersonCharacter OtherActor))
  (Variables|/Game/ThirdPerson/Blueprints/BP_ThirdPersonCharacter.BP_ThirdPersonCharacter_C|SetDoor%20 _asbp_third_person_character self)
  (Variables|Default|SetTouching true)
  (Variables|Default|SetPlayer _asbp_third_person_character))

(event OnComponentEndOverlap(Box)
  (params (OverlappedComponent :type Primitive%20Component%20Object%20Reference) (OtherActor :type Actor%20Object%20Reference) (OtherComp :type Primitive%20Component%20Object%20Reference) (OtherBodyIndex :type Integer))
  (Utilities|Casting|CastToBP_ThirdPersonCharacter OtherActor)
  (Variables|Default|SetTouching false))

(event Custom|Open%20Door
  (bind _returnvalue (Game|GetPlayerController 0))
  (bind _player (Variables|Default|GetPlayer))
  (bind _spawncard (Variables|Default|GetSpawnCard))
  (if (Variables|Default|GetFake%20Door)
    (bind _returnvalue_2 (Game|ConstructObjectfromClass "/Game/ActualGame/UI/LoseMenu.LoseMenu_C"))
    (UserInterface|Viewport|AddtoViewport _returnvalue_2 0)
    (Variables|/Script/Engine.PlayerController|SetbShowMouseCursor _returnvalue true)
    (Input|SetInputModeUIOnly _returnvalue 0 "DoNotLock" false)
    (Actor|DestroyActor)
    (else
      (Transformation|Teleport _player (Transformation|GetActorLocation (Variables|Default|GetWaypoint)) "0, 0, 0")
      (Default|RemoveItem _player)
      (Utilities|IsValid (Variables|Default|GetWaypoint)
        (:Is%20Valid
          (Utilities|IsValid _spawncard
            (:Is%20Valid
              (Game|SpawnActorfromClass "/Game/ActualGame/BluePrints/BP_CardPickUp.BP_CardPickUp_C" (Transformation|GetActorTransform _spawncard) "Undefined" "MultiplyWithRoot" 0 0))
            (:Is%20Not%20Valid
              _)))
        (:Is%20Not%20Valid
          _))
      (Actor|DestroyActor))))

(event EventBeginPlay)

(event Collision|EventActorBeginOverlap
  (params (OtherActor :type Actor%20Object%20Reference)))

(event EventTick
  (params (DeltaSeconds :type Float%20%28single-precision%29)))

(fn ConstructionScript)