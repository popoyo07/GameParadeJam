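; BP_Squicky is an interactable actor that plays a squeak sound when the player presses E while inside its sphere.
; Sphere overlap events track whether a BP_ThirdPersonCharacter is touching it and cache that character.
; Tick polls the character's PressedE flag, using a PlayingSound latch to fire the 2D sound once until E is released or the overlap ends.
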(event OnComponentBeginOverlap(Sphere)
  (params (OverlappedComponent :type Primitive%20Component%20Object%20Reference) (OtherActor :type Actor%20Object%20Reference) (OtherComp :type Primitive%20Component%20Object%20Reference) (OtherBodyIndex :type Integer) (bFromSweep :type Boolean) (SweepResult :type Hit%20Result%20Structure%20%28by%20ref%29))
  (bind _asbp_third_person_character (Utilities|Casting|CastToBP_ThirdPersonCharacter OtherActor))
  (Variables|Default|SetTouching%20Switch true)
  (Development|PrintString "Touching")
  (Variables|Default|SetCharacter _asbp_third_person_character))

(event OnComponentEndOverlap(Sphere)
  (params (OverlappedComponent :type Primitive%20Component%20Object%20Reference) (OtherActor :type Actor%20Object%20Reference) (OtherComp :type Primitive%20Component%20Object%20Reference) (OtherBodyIndex :type Integer))
  (Utilities|Casting|CastToBP_ThirdPersonCharacter OtherActor)
  (Variables|Default|SetTouching%20Switch false)
  (Development|PrintString "Not touching"))

(event EventBeginPlay)

(event Collision|EventActorBeginOverlap
  (params (OtherActor :type Actor%20Object%20Reference)))

(event EventTick
  (params (DeltaSeconds :type Float%20%28single-precision%29))
  (bind _character (Variables|Default|GetCharacter))
  (Utilities|IsValid _character
    (:Is%20Valid
      (if (Variables|/Game/ThirdPerson/Blueprints/BP_ThirdPersonCharacter.BP_ThirdPersonCharacter_C|GetPressed%20E _character)
        (if (Variables|Default|GetTouching%20Switch)
          (if (not (Variables|Default|GetPlaying%20sound%20))
            (Audio|PlaySound2D "/Game/ActualGame/Sound/Squeak.Squeak" 1.0 1.0 0.0 0 0)
            (Variables|Default|SetPlaying%20sound%20 true))
          (else
            (Variables|Default|SetPlaying%20sound%20 false :!label _label)))
        (else
          (goto _label))))
    (:Is%20Not%20Valid
      (goto _label))))

(fn ConstructionScript)