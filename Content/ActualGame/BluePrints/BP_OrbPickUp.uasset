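; BP_OrbPickUp is an orb pickup that the third-person character can collect.
; Sphere overlap caches the character, registers the orb as its ItemPickUp and sets IsTouching, with no end-overlap handling to clear them.
; Interact marks the character as holding the orb instead of the card or gun, returns the orb's static mesh and triggers destruction after a short delay.
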(event OnComponentBeginOverlap(Sphere)
  (params (OverlappedComponent :type Primitive%20Component%20Object%20Reference) (OtherActor :type Actor%20Object%20Reference) (OtherComp :type Primitive%20Component%20Object%20Reference) (OtherBodyIndex :type Integer) (bFromSweep :type Boolean) (SweepResult :type Hit%20Result%20Structure%20%28by%20ref%29))
  (bind _asbp_third_person_character (Utilities|Casting|CastToBP_ThirdPersonCharacter OtherActor))
  (Variables|Default|SetPCharacter _asbp_third_person_character)
  (Development|PrintString "SHOULD INTERACT")
  (Variables|/Game/ThirdPerson/Blueprints/BP_ThirdPersonCharacter.BP_ThirdPersonCharacter_C|SetItemPickUp (Variables|Default|GetPCharacter) self)
  (Variables|/Game/ThirdPerson/Blueprints/BP_ThirdPersonCharacter.BP_ThirdPersonCharacter_C|SetIsTouching (Variables|Default|GetPCharacter) true))

(event Custom|Destroy%20Item
  (Utilities|FlowControl|Delay 0.2)
  (Actor|DestroyActor))

(event EventBeginPlay)

(event EventTick
  (params (DeltaSeconds :type Float%20%28single-precision%29)))

(fn ConstructionScript)

(fn Interact
  (bind _pcharacter (Variables|Default|GetPCharacter))
  (Utilities|IsValid (Variables|Default|GetPCharacter)
    (:Is%20Valid
      (Development|PrintString "picked up Orb")
      (CallFunction|DestroyItem)
      (Variables|/Game/ThirdPerson/Blueprints/BP_ThirdPersonCharacter.BP_ThirdPersonCharacter_C|SetHasOrb _pcharacter true)
      (Variables|/Game/ThirdPerson/Blueprints/BP_ThirdPersonCharacter.BP_ThirdPersonCharacter_C|SetHasCard _pcharacter false)
      (Variables|/Game/ThirdPerson/Blueprints/BP_ThirdPersonCharacter.BP_ThirdPersonCharacter_C|SetHasGun _pcharacter false)
      (return (Variables|/Script/Engine.StaticMeshComponent|GetStaticMesh (Variables|Default|GetStaticMesh))))
    (:Is%20Not%20Valid
      (Development|PrintString "SHOULD NOT INTERACT"))))