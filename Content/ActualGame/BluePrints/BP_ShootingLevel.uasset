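; BP_ShootingLevel runs a shooting challenge that the player must clear with a limited number of bullets.
; Its Detect component latches a flag when the third-person character overlaps it and counts each overlapping BP_Bullet.
; Once flagged, Tick opens GameLevel as a loss at the shot limit, or destroys this actor when HitTarget reaches its goal.
; HitTarget is only read here, never incremented.
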(event OnComponentBeginOverlap(Detect)
  (params (OverlappedComponent :type Primitive%20Component%20Object%20Reference) (OtherActor :type Actor%20Object%20Reference) (OtherComp :type Primitive%20Component%20Object%20Reference) (OtherBodyIndex :type Integer) (bFromSweep :type Boolean) (SweepResult :type Hit%20Result%20Structure%20%28by%20ref%29))
  (Development|PrintString "overlap")
  (Utilities|Casting|CastToBP_ThirdPersonCharacter OtherActor
    (:then
      (bind _output_get (Variables|Default|Setoverlap%20Player true)))
    (:CastFailed
      ;[0.15 0.15 0.15 0.5] Bullet counter
      (Utilities|Casting|CastToBP_Bullet OtherActor)
      (Variables|Default|SetBulletsShot (+ (Variables|Default|GetBulletsShot) 1)))))

(event EventBeginPlay)

(event Collision|EventActorBeginOverlap
  (params (OtherActor :type Actor%20Object%20Reference)))

(event EventTick
  (params (DeltaSeconds :type Float%20%28single-precision%29))
  (if (stale OnComponentBeginOverlap(Detect) _output_get)
    (if (== (Variables|Default|GetBulletsShot) 25)
      ;[0.15 0.15 0.15 0.5] LoseLogic
      (Game|OpenLevel(byName) "GameLevel")
      (else
        (Development|PrintString (Utilities|String|ToString(Integer) (Variables|Default|GetHitTarget)))
        ;[0.15 0.15 0.15 0.5] Place door bp reference after this
        (if (== (Variables|Default|GetHitTarget) 6)
          (Actor|DestroyActor))))))

(fn ConstructionScript)